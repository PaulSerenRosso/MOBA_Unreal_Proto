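; AI controller for melee enemies that runs BT_MeleeEnemy on the server and enables its CanAttack blackboard flag.
; Every tick and perception event rebuilds targets from known perceived actors, keeping only melee enemies and champion characters.
; The current target stays while still listed, otherwise the first takes over, and the Blackboard Target key follows or clears.
; Team checking via IsEnemy appears only in disconnected logic, so live targeting ignores teams.
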(event OnTargetPerceptionUpdated(AIPerception)
  (params (Actor :type Actor%20Object%20Reference) (Stimulus :type AI%20Stimulus%20Structure))
  (CallFunction|UpdatedPerception))

(event OnPerceptionUpdated(AIPerception)
  (params (UpdatedActors :type Array%20of%20Actor%20Object%20References))
  (CallFunction|UpdatedPerception))

(event OnTargetPerceptionForgotten(AIPerception)
  (params (Actor :type Actor%20Object%20Reference))
  (CallFunction|UpdatedPerception))

(event Custom|UpdatedPerception
  (params (Actor :type Actor%20Object%20Reference) (Stimulus :type AI%20Stimulus%20Structure))
  (Utilities|IsValid (Variables|Default|GetBlackboard)
    (:Is%20Valid
      (CallFunction|MakeTargets (Class|AIPerceptionComponent|GetKnownPerceivedActors (Variables|Default|GetAIPerception)))
      (bind _filteredarray (Utilities|Array|FilterArray (Variables|Default|GetTrueTargets) "/Script/Engine.Pawn"))
      (if (Utilities|Array|IsNotEmpty _filteredarray)
        (if (Utilities|Array|ContainsItem _filteredarray (Variables|Default|GetTargetActor))
          (if (Utilities|IsValid (Variables|Default|GetTargetActor))
            (AI|Components|Blackboard|SetValueasObject (Variables|Default|GetBlackboard) (Utilities|Name|MakeLiteralName "Target") (Variables|Default|GetTargetActor))
            (else
              (bind _output_get (Variables|Default|SetTargetActor (Utilities|Array|Get(acopy) _filteredarray) :!label _label))
              (AI|Components|Blackboard|SetValueasObject (Variables|Default|GetBlackboard) (Utilities|Name|MakeLiteralName "Target") _output_get)))
          (else
            (goto _label)))
        (else
          (Variables|Default|SetTargetActor 0)
          (AI|Components|Blackboard|SetValueasObject (Variables|Default|GetBlackboard) (Utilities|Name|MakeLiteralName "Target") 0))))))

(event Custom|MakeTargets
  (params (NewParam :type Array%20of%20Actor%20Object%20References))
  (Utilities|Array|Clear (Variables|Default|GetTrueTargets))
  (for _array_element NewParam
    ;[1 1 1] Should be implement interface
    (Utilities|Casting|CastToBP_MeleeEnemy _array_element
      (:then
        _)
      (:CastFailed
        (Utilities|Casting|CastToBP_ChampionCharacter _array_element)))
    (Utilities|Array|AddUnique (Variables|Default|GetTrueTargets) _array_element)))

(event Custom|Run%20Behavior%20Tree
  (Networking|SwitchHasAuthority
    (:Authority
      (AI|RunBehaviorTree "/Game/AI/BT_MeleeEnemy.BT_MeleeEnemy")
      (CallFunction|SetCanAttack true))))

(event EventTick
  (params (DeltaSeconds :type Float%20%28single-precision%29))
  (CallFunction|UpdatedPerception))

(fn ConstructionScript)

(fn IsEnemy
  (params (Team%20pawn1 :type ETeam%20Enum :default "Neutral") (Team%20pawn2 :type ETeam%20Enum :default "Neutral"))
  (if (Utilities|Enum|Equal(Enum) Team%20pawn1 "Neutral")
    _
    (elif (Utilities|Enum|Equal(Enum) Team%20pawn2 "Neutral")
      _
      (else
        (return (Utilities|Enum|NotEqual(Enum) Team%20pawn1 Team%20pawn2)))))
  (return false))

(fn SetCanAttack
  (params (Value :type Boolean))
  (Utilities|IsValid (Variables|Default|GetBlackboard)
    (:Is%20Valid
      (AI|Components|Blackboard|SetValueasBool (Variables|Default|GetBlackboard) (Utilities|Name|MakeLiteralName "CanAttack") Value))))
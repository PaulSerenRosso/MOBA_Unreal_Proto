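; BP_MeleeEnemy is a team-based melee enemy that shows its health on a widget bar.
; On BeginPlay it fills health and applies its team material from BP_GameModeBattle, tinting the bar blue or red.
; Health, player-join and sync events refresh the bar and rotate it toward the player camera only at that moment.
; A helper queries random reachable points around a target; attack logic is absent here.
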(event Custom|SychronizeHealthTo
  (params (HealthToSync :type Integer))
  (Variables|Default|SetCurrentHealth HealthToSync)
  (CallFunction|UpdateCharHealth))

(event Custom|SyncFromServer
  (CallFunction|SychronizeHealthto (Variables|Default|GetCurrentHealth)))

(event EventBeginPlay
  (CallFunction|ChangeTeam)
  (Variables|Default|SetCurrentHealth (Variables|Default|GetMaxHealth)))

(event Collision|EventActorBeginOverlap
  (params (OtherActor :type Actor%20Object%20Reference)))

(event EventOnPlayerJoin
  (Development|PrintString "Player Join")
  (CallFunction|UpdateCharHealth))

(event EventChangedTeam
  (CallFunction|ChangeTeam))

(event EventUpdateHealth
  (CallFunction|UpdateCharHealth))

(fn ConstructionScript
  (Variables|Default|SetMeshComponent (Variables|Character|GetMesh))
  (CallFunction|UpdateCharHealth))

(fn FindPointAroundTarget
  (params (Target :type Vector :default "0, 0, 0") (Radius :type Float%20%28single-precision%29))
  (bind (_randomlocation _returnvalue) (AI|Navigation|GetRandomReachablePointinRadius Target Radius 0 0))
  (Variables|Default|SettargetLocation _randomlocation)
  (return _returnvalue))

(fn ChangeTeam
  (bind _asbp_game_mode_battle (Utilities|Casting|CastToBP_GameModeBattle (Game|GetGameMode))
    (:then
      (bind _returnvalue (Class|GameModeBattle|GetTeamMaterial _asbp_game_mode_battle (Variables|Default|GetTeam)))
      (Rendering|Material|SetMaterial (Variables|Default|GetMeshComponent) 1 _returnvalue)
      (bind _aswbp_health_bar (Utilities|Casting|CastToWBP_HealthBar (UserInterface|GetWidget (Variables|Default|GetWidget))))
      (switch Utilities|FlowControl|Switch|SwitchonETeam (Variables|Default|GetTeam)
        (:Team1
          (Class|ProgressBar|SetFillColorandOpacity (Variables|/Game/Blueprints/UI/WBP_HealthBar.WBP_HealthBar_C|GetHealth _aswbp_health_bar) "(R=0.000000,G=0.046308,B=1.000000,A=1.000000)"))
        (:Team2
          (Class|ProgressBar|SetFillColorandOpacity (Variables|/Game/Blueprints/UI/WBP_HealthBar.WBP_HealthBar_C|GetHealth _aswbp_health_bar) "(R=0.741666,G=0.000000,B=0.020016,A=1.000000)"))))
    (:CastFailed
      (Development|PrintString "Failed to cast"))))

(fn UpdateCharHealth
  (bind _aswbp_health_bar (Utilities|Casting|CastToWBP_HealthBar (UserInterface|GetWidget (Variables|Default|GetWidget)))
    (:then
      (bind _returnvalue (Class|EnemyBase|GetPercentHealth))
      (Default|UpdateHealth _aswbp_health_bar _returnvalue)
      (Transformation|SetWorldRotation (Variables|Default|GetWidget) (Math|Rotator|FindLookatRotation (Transformation|GetWorldLocation (Variables|Default|GetWidget)) (Transformation|GetWorldLocation (Variables|/Script/Engine.PlayerCameraManager|GetTransformComponent (Game|GetPlayerCameraManager 0)))) false false)
      (return))
    (:CastFailed
      (return))))
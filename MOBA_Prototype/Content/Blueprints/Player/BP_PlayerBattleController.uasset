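; BP_PlayerBattleController manages the on-screen cursor widget for the player's battle controller.
; On begin play, it creates a WBP_Cursor widget for the first player controller, only when the owning-client check passes.
; Owner-client activation and deactivation events for the battle character add the cursor to the viewport and remove it again.
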(event EventBeginPlay
  (bind _returnvalue (Class|PlayerBattleController|CheckOwningClient))
  (if _returnvalue
    (bind _returnvalue_2 (UserInterface|CreateWidget "/Game/Blueprints/UI/WBP_Cursor.WBP_Cursor_C" (Game|GetPlayerController 0)))
    (Variables|Default|SetCursorWidget _returnvalue_2)))

(event EventOnActivateBattleCharacterClientOwner
  (UserInterface|Viewport|AddtoViewport (Variables|Default|GetCursorWidget) 0))

(event EventOnDeactivateBattleCharacterClientOwner
  (Widget|RemovefromParent (Variables|Default|GetCursorWidget)))

(fn ConstructionScript)